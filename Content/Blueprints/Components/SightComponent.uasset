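; Actor component for a Unit that records, per team, whether the unit is visible to that team.
; A CheckInit macro lazily fills the Sights array on first access, marking only the owner's own team as visible.
; SetSight writes the flag by team index and first dispatches a byte event on the owning Unit when a team loses sight.
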(event EventBeginPlay)

(event EventTick
  (params (DeltaSeconds :type Float%20%28single-precision%29)))

(fn SetSight
  (params (Team :type bp_Team%20Enum :default "NewEnumerator0") (Visible :type Boolean))
  (Utilities|CheckInit
    (:Inited
      (bind _visible (CallFunction|GetSight Team))
      (if (and _visible (Math|Boolean|Equal(Boolean) Visible false))
        (bind _asunit (Utilities|Casting|CastToUnit (Components|GetOwner)))
        (Default|DispatchByteEvent _asunit "NewEnumerator0" Team))
      (Utilities|Array|SetArrayElem (Variables|Default|GetSights) (Math|Conversions|ToInteger(Byte) Team) Visible))))

(fn GetSight
  (params (Team :type bp_Team%20Enum :default "NewEnumerator0"))
  (Utilities|CheckInit
    (:Inited
      (return (Utilities|Array|Get(acopy) (Variables|Default|GetSights) (Math|Conversions|ToInteger(Byte) Team))))))

(fn Init
  (Utilities|FlowControl|Sequence
    (:then_0
      (|ForEachbp_Team
        (:LoopBody
          (Utilities|Array|Add (Variables|Default|GetSights) false))))
    (:then_1
      (bind _asunit (Utilities|Casting|CastToUnit (Components|GetOwner)))
      (CallFunction|SetSight (Variables|/Game/Blueprints/Units/Unit.Unit_C|GetTeam _asunit) true))))