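; Game mode for a team MOBA that runs battles from player login to Nexus death.
; The first login sets up fountains, UnitFactory and MinionSpawner; each player gets a champion on alternating teams, with post-login triggered from C++ for UEtopia.
; A GameInstance MatchInfo ready check drives GameState's battle state, which resets units, opens fountains and toggles minion spawning.
; Nexus death ends the battle, announces victory and records the win through GameInstance.
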(event Custom|ResetGame
  ;[1 1 1] ResetGame
  (Utilities|OpenFountain false)
  (Default|DestroyAllUnits (Variables|Default|GetUnitFactory))
  (Utilities|SpawnTargetPointUnitsandSetEventtoNexus
    (:Set
      (bind _myplayerstate (Utilities|GetAllMyPlayerState)
        (:LoopBody
          (bind _transform (CallFunction|GetSpawnTransform (Variables|/Game/Blueprints/PlayerState/bp_MyPlayerState.bp_MyPlayerState_C|GetTeam _myplayerstate)))
          (Default|SpawnUnit (Variables|Default|GetUnitFactory) (Variables|/Game/Blueprints/PlayerState/bp_MyPlayerState.bp_MyPlayerState_C|GetTeam _myplayerstate) (Variables|/Game/Blueprints/PlayerState/bp_MyPlayerState.bp_MyPlayerState_C|GetChampionKey _myplayerstate) _transform "AdjustIfPossibleButAlwaysSpawn" (Variables|/Game/Blueprints/PlayerState/bp_MyPlayerState.bp_MyPlayerState_C|GetPlayerController _myplayerstate))
          (Variables|/Game/Blueprints/PlayerState/bp_MyPlayerState.bp_MyPlayerState_C|SetReady _myplayerstate false))))))

(event Custom|SetBattleState
  (params (NewBattleState :type BattleState%20Enum :default "NewEnumerator0"))
  ;[1 1 1] SetBattleState
  (bind _asbp_my_game_state (Utilities|Casting|CastTobp_MyGameState (Game|GetGameState)))
  (bind _output_get (Variables|/Game/Blueprints/GameState/bp_MyGameState.bp_MyGameState_C|SetBattleState _asbp_my_game_state NewBattleState))
  (switch Utilities|FlowControl|Switch|SwitchonBattleState _output_get
    (:NewEnumerator0
      (CallFunction|ResetGame)
      (CallFunction|SetCenterTexttoAllClient "Prepare for Battle" 96 (Utilities|Struct|MakeSlateColor "(R=1.000000,G=1.000000,B=1.000000,A=1.000000)") 4.0))
    (:NewEnumerator1
      (Utilities|OpenFountain true)
      (Default|SetSpawn (Variables|Default|GetMinionSpawner) true)
      (CallFunction|SetCenterTexttoAllClient "Battle Start" 96 (Utilities|Struct|MakeSlateColor "(R=1.000000,G=1.000000,B=1.000000,A=1.000000)") 4.0))
    (:NewEnumerator2
      (Default|DisableAllUnits (Variables|Default|GetUnitFactory))
      (Default|SetSpawn (Variables|Default|GetMinionSpawner) false))))

(event Custom|RedyCheck
  ;[1 1 1] Ready Check - UETOPIA CHANGES - Using GameInstance Match info instead
  (Development|PrintString "bp_MyGameMode RedyCheck")
  (Variables|Default|SetAllReady true)
  (bind _asmy_game_instance (Utilities|Casting|CastToMyGameInstance (Game|GetGameInstance)))
  (for _array_element (.players (Utilities|Struct|BreakMyMatchInfo (Variables|/Script/OpenMOBA.MyGameInstance|GetMatchInfo _asmy_game_instance)))
    (if (not (.characterCustomized (Utilities|Struct|BreakMyMatchPlayer _array_element)))
      (Variables|Default|SetAllReady false)))
  (Development|PrintString "Redy check finished scanning players")
  (if (Variables|Default|GetAllReady)
    (CallFunction|SetBattleState "NewEnumerator1")
    (Development|PrintString "bp_MyGameMode InBattle")
    (Utilities|FlowControl|Delay 5.0)
    (bind _myplayerstate (Utilities|GetAllMyPlayerState)
      (:LoopBody
        (Class|MyPlayerState|OnReponCustomTextureChange _myplayerstate)))
    (else
      (CallFunction|SetBattleState "NewEnumerator0")
      (Development|PrintString "bp_MyGameMode BeforeBattle"))))

(event Custom|Init
  ;[1 1 1] Init
  (Development|PrintString "bp_MyGameMode_Init")
  (Utilities|FlowControl|Sequence
    (:then_0
      (bind _outactors (Actor|GetAllActorsOfClass "/Game/Blueprints/Fountain/Fountain.Fountain_C"))
      (for _array_element _outactors
        (Utilities|Map|Add (Variables|Default|GetFountains) (Variables|/Game/Blueprints/Fountain/Fountain.Fountain_C|GetTeam _array_element) _array_element)
        (Default|SetOpen _array_element false)
        (CallFunction|SetBattleState "NewEnumerator0")))
    (:then_1
      (Utilities|IsValid (Variables|Default|GetUnitFactory)
        (:Is%20Valid
          _)
        (:Is%20Not%20Valid
          (bind _returnvalue (Game|SpawnActorfromClass "/Game/Blueprints/GameMode/UnitFactory/UnitFactory.UnitFactory_C" (Math|Transform|MakeTransform "0, 0, 0") "AlwaysSpawn" 0 0))))
      (bind _output_get (Variables|Default|SetUnitFactory _returnvalue))
      (Default|Init _output_get))
    (:then_2
      (Utilities|IsValid (Variables|Default|GetMinionSpawner)
        (:Is%20Valid
          _)
        (:Is%20Not%20Valid
          (bind _returnvalue_2 (Game|SpawnActorfromClass "/Game/Blueprints/GameMode/MinionSpawner/MinionSpawner.MinionSpawner_C" (Math|Transform|MakeTransform "0, 0, 0") "AlwaysSpawn" 0 0))))
      (bind _output_get_2 (Variables|Default|SetMinionSpawner _returnvalue_2))
      (Default|Init _output_get_2 (Variables|Default|GetUnitFactory))
      (Default|SetSpawn _output_get_2 false))
    (:then_3
      (Utilities|SpawnTargetPointUnitsandSetEventtoNexus))))

(event Custom|ChangeChampion
  (params (PlayerController :type Player%20Controller%20Object%20Reference) (ChampionKeyName :type Name))
  ;[1 1 1] ChangeChampion
  (bind _asbp_my_player_controller (Utilities|Casting|CastTobp_MyPlayerController PlayerController))
  (bind _output_get (Variables|Default|SetPreviousTeam (Variables|/Game/Blueprints/Units/Unit.Unit_C|GetTeam (Variables|/Game/Blueprints/PlayerController/bp_MyPlayerController.bp_MyPlayerController_C|GetCommandUnit _asbp_my_player_controller))))
  (Actor|DestroyActor (Variables|/Game/Blueprints/PlayerController/bp_MyPlayerController.bp_MyPlayerController_C|GetCommandUnit _asbp_my_player_controller))
  (bind _transform (CallFunction|GetSpawnTransform _output_get))
  (Default|SpawnUnit (Variables|Default|GetUnitFactory) (Variables|Default|GetPreviousTeam) ChampionKeyName _transform "AdjustIfPossibleButAlwaysSpawn" PlayerController))

(event Custom|RecallUnit
  (params (Unit :type Unit%20Object%20Reference))
  ;[1 1 1] RecallUnit
  (bind _transform (CallFunction|GetSpawnTransform (Variables|/Game/Blueprints/Units/Unit.Unit_C|GetTeam Unit)))
  (Transformation|SetActorTransform Unit _transform))

(event Custom|SetNexusDeathEvent
  ;[1 1 1] SetNexusDeathEvent
  (bind _outactors (Actor|GetAllActorsOfClass "/Game/Blueprints/Units/ImmobileUnit/Nexus/Nexus.Nexus_C"))
  (for _array_element _outactors
    (bind _wrapper (Default|GetNormalEventDispatcher _array_element "NewEnumerator0"))
    (EventDispatchers|BindEventtoWrappedEventDispatcher _wrapper (delegate Custom|OnDeath))))

(event Custom|OnDeath
  (params (Actor :type Actor%20Object%20Reference))
  ;[1 1 1] SetNexusDeathEvent
  (bind _asunit (Utilities|Casting|CastToUnit Actor))
  (if (Utilities|Enum|Equal(Enum) (Variables|/Game/Blueprints/Units/Unit.Unit_C|GetTeam _asunit) "NewEnumerator2")
    (Variables|Default|SetWinningTeamId 1)
    (else
      (Variables|Default|SetWinningTeamId 0)))
  (CallFunction|SetCenterTexttoAllClient "Victory" 128 (select (Utilities|Enum|Equal(Enum) (Variables|/Game/Blueprints/Units/Unit.Unit_C|GetTeam _asunit) "NewEnumerator2") (Utilities|Struct|MakeSlateColor "(R=0.000000,G=0.000000,B=1.000000,A=1.000000)") (Utilities|Struct|MakeSlateColor "(R=1.000000,G=0.000000,B=0.000000,A=1.000000)")) 0.0)
  (CallFunction|SetBattleState "NewEnumerator2")
  ;[1 1 1] Record the WIN, which will update ranks, and save the data to the backend
  (bind _asmy_game_instance (Utilities|Casting|CastToMyGameInstance (Game|GetGameInstance)))
  (Class|MyGameInstance|RecordRoundWin _asmy_game_instance (Variables|Default|GetWinningTeamId)))

(event Custom|ChangeTeam
  (params (PlayerController :type Player%20Controller%20Object%20Reference) (Team :type bp_Team%20Enum :default "NewEnumerator0"))
  ;[1 1 1] ChangeTeam
  (bind _asbp_my_player_controller (Utilities|Casting|CastTobp_MyPlayerController PlayerController))
  (Variables|Default|SetPreviousChampionKey (Variables|/Game/Blueprints/Units/Unit.Unit_C|GetUnitKey (Variables|/Game/Blueprints/PlayerController/bp_MyPlayerController.bp_MyPlayerController_C|GetCommandUnit _asbp_my_player_controller)))
  (Actor|DestroyActor (Variables|/Game/Blueprints/PlayerController/bp_MyPlayerController.bp_MyPlayerController_C|GetCommandUnit _asbp_my_player_controller))
  (bind _transform (CallFunction|GetSpawnTransform Team))
  (Default|SpawnUnit (Variables|Default|GetUnitFactory) Team (Variables|Default|GetPreviousChampionKey) _transform "AdjustIfPossibleButAlwaysSpawn" PlayerController))

(event Custom|SetCenterTextToAllClient
  (params (Text :type Text) (FontSize :type Integer) (Color :type Slate%20Color%20Structure) (Duration :type Float%20%28single-precision%29))
  ;[1 1 1] SetCenterTextToAllClient
  (bind _myplayerstate (Utilities|GetAllMyPlayerState)
    (:LoopBody
      (bind _asbp_my_player_controller (Utilities|Casting|CastTobp_MyPlayerController (Variables|/Game/Blueprints/PlayerState/bp_MyPlayerState.bp_MyPlayerState_C|GetPlayerController _myplayerstate)))
      (Default|SetCenterTextWidget _asbp_my_player_controller Text FontSize Color Duration))))

(event EventBeginPlay
  (Development|PrintString "bp_MyGameMode Begin Play"))

(event EventTick
  (params (DeltaSeconds :type Float%20%28single-precision%29)))

(event EventPostLogin
  (params (NewPlayer :type Player%20Controller%20Object%20Reference))
  ;[1 1 1] OnPostLogin
  (Development|PrintString "bp_myGameMode_OnPostLogin")
  (if (not (Variables|Default|GetInitFlag))
    (Variables|Default|SetInitFlag true)
    (CallFunction|Init))
  (bind _output_get (Variables|Default|SetNewPlayer (stale EventEventOnPostLogin NewPlayerController)))
  (bind _asbp_my_player_controller (Utilities|Casting|CastTobp_MyPlayerController _output_get)
    (:then
      (Default|Init _asbp_my_player_controller)
      (Utilities|FlowControl|FlipFlop
        (:A
          (Variables|Default|SetSpawnTeam "NewEnumerator1"))
        (:B
          (Variables|Default|SetSpawnTeam "NewEnumerator2")))
      (bind _transform (CallFunction|GetSpawnTransform (Variables|Default|GetSpawnTeam)))
      (Default|SpawnUnit (Variables|Default|GetUnitFactory) (Variables|Default|GetSpawnTeam) (Variables|Default|GetDefaultChampionKey) _transform "AdjustIfPossibleButAlwaysSpawn" (Variables|Default|GetNewPlayer))
      (bind _playerstate (CallFunction|GetPlayerState (Variables|Default|GetNewPlayer)))
      (CallFunction|SetPlayerState (Variables|Default|GetNewPlayer) (Variables|/Game/Blueprints/PlayerState/bp_MyPlayerState.bp_MyPlayerState_C|GetCustomeName _playerstate) (Variables|Default|GetSpawnTeam) (Variables|Default|GetDefaultChampionKey) false)
      (CallFunction|RedyCheck))
    (:CastFailed
      (Development|PrintString "b-PMyGameMode cast to bp_MyPlayerController FAIL")
      (Utilities|Casting|CastToMyPlayerController _output_get
        (:then
          (Development|PrintString "Cast to MyPlayerController success"))
        (:CastFailed
          (Development|PrintString "Cast to MyPlayerController fail"))))))

(event EventOnLogout
  (params (ExitingController :type Controller%20Object%20Reference))
  ;[1 1 1] OnLogout
  (bind _asbp_my_player_controller (Utilities|Casting|CastTobp_MyPlayerController ExitingController))
  (Utilities|IsValid (Variables|/Game/Blueprints/PlayerController/bp_MyPlayerController.bp_MyPlayerController_C|GetCommandUnit _asbp_my_player_controller)
    (:Is%20Valid
      (Actor|DestroyActor (Variables|/Game/Blueprints/PlayerController/bp_MyPlayerController.bp_MyPlayerController_C|GetCommandUnit _asbp_my_player_controller)))))

(event EventEventOnPostLogin
  (params (NewPlayerController :type Player%20Controller%20Object%20Reference))
  ;[1 1 1] UETOPIA CHANGES - OnPostLogin is never called so we call this manually from c++
  (Development|PrintString "bp_myGameMode_RecieveEventOnPostLogin")
  ;[1 1 1] OnPostLogin
  (if (not (Variables|Default|GetInitFlag))
    (Variables|Default|SetInitFlag true)
    (CallFunction|Init))
  (bind _output_get (Variables|Default|SetNewPlayer NewPlayerController))
  (bind _asbp_my_player_controller (Utilities|Casting|CastTobp_MyPlayerController _output_get)
    (:then
      (Default|Init _asbp_my_player_controller)
      (Utilities|FlowControl|FlipFlop
        (:A
          (Variables|Default|SetSpawnTeam "NewEnumerator1"))
        (:B
          (Variables|Default|SetSpawnTeam "NewEnumerator2")))
      (bind _transform (CallFunction|GetSpawnTransform (Variables|Default|GetSpawnTeam)))
      (Default|SpawnUnit (Variables|Default|GetUnitFactory) (Variables|Default|GetSpawnTeam) (Variables|Default|GetDefaultChampionKey) _transform "AdjustIfPossibleButAlwaysSpawn" (Variables|Default|GetNewPlayer))
      (bind _playerstate (CallFunction|GetPlayerState (Variables|Default|GetNewPlayer)))
      (CallFunction|SetPlayerState (Variables|Default|GetNewPlayer) (Variables|/Game/Blueprints/PlayerState/bp_MyPlayerState.bp_MyPlayerState_C|GetCustomeName _playerstate) (Variables|Default|GetSpawnTeam) (Variables|Default|GetDefaultChampionKey) false)
      (CallFunction|RedyCheck))
    (:CastFailed
      (Development|PrintString "b-PMyGameMode cast to bp_MyPlayerController FAIL")
      (Utilities|Casting|CastToMyPlayerController _output_get
        (:then
          (Development|PrintString "Cast to MyPlayerController success"))
        (:CastFailed
          (Development|PrintString "Cast to MyPlayerController fail"))))))

(fn ConstructionScript)

(fn SetPlayerState
  (params (PlayerController :type Player%20Controller%20Object%20Reference) (CustomeName :type String) (Team :type bp_Team%20Enum :default "NewEnumerator0") (ChampionKeyName :type Name) (Ready :type Boolean))
  (bind _asbp_my_player_state (Utilities|Casting|CastTobp_MyPlayerState (Variables|/Script/Engine.Controller|GetPlayerState PlayerController)))
  (Utilities|FlowControl|Sequence
    (:then_0
      (Variables|/Game/Blueprints/PlayerState/bp_MyPlayerState.bp_MyPlayerState_C|SetPlayerController _asbp_my_player_state PlayerController))
    (:then_1
      (Variables|/Game/Blueprints/PlayerState/bp_MyPlayerState.bp_MyPlayerState_C|SetCustomeName _asbp_my_player_state CustomeName))
    (:then_2
      (Variables|/Game/Blueprints/PlayerState/bp_MyPlayerState.bp_MyPlayerState_C|SetTeam _asbp_my_player_state Team))
    (:then_3
      (Variables|/Game/Blueprints/PlayerState/bp_MyPlayerState.bp_MyPlayerState_C|SetChampionKey _asbp_my_player_state ChampionKeyName))
    (:then_4
      (Variables|/Game/Blueprints/PlayerState/bp_MyPlayerState.bp_MyPlayerState_C|SetReady _asbp_my_player_state Ready))))

(fn GetPlayerState
  (params (PlayerController :type Player%20Controller%20Object%20Reference))
  (bind _asbp_my_player_state (Utilities|Casting|CastTobp_MyPlayerState (Variables|/Script/Engine.Controller|GetPlayerState PlayerController)))
  (return _asbp_my_player_state))

(fn GetSpawnTransform
  (params (Team :type bp_Team%20Enum :default "NewEnumerator0"))
  (bind _transform (Default|GetSpawnTransform (.Value (Utilities|Map|Find (Variables|Default|GetFountains) Team))))
  (return _transform))