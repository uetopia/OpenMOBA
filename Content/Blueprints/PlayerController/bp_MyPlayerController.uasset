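; MOBA player controller that commands a replicated CommandUnit, manages its camera and opens HUD widgets.
; Mouse traces become attack (visible living enemies), move or attack-move commands via SetCommand, alongside recall.
; Champion inventory events handle item use, selling, and buying near a team fountain with data-table prices.
; OnRep_CommandUnit spawns the local ClientCamera for scroll, zoom and follow; player-state setup carries UEtopia edits.
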(event Custom|SendConsumeItem
  (params (Index :type Integer))
  ;[1 1 1] SendConsumeItem
  (if (Utilities|IsCommandUnitValid)
    (bind _aschampion (Utilities|Casting|CastToChampion (Variables|Client&Server|GetCommandUnit)))
    (Default|Consume (Variables|/Game/Blueprints/Units/MobileUnit/Champions/Champion.Champion_C|GetInventoryComponent _aschampion) Index)))

(event Custom|SellItem
  (params (Index :type Integer))
  ;[1 1 1] SellItem
  (if (Utilities|IsCommandUnitValid)
    (bind _aschampion (Utilities|Casting|CastToChampion (Variables|Client&Server|GetCommandUnit)))
    (bind _itemkey (Default|GetItem (Variables|/Game/Blueprints/Units/MobileUnit/Champions/Champion.Champion_C|GetInventoryComponent _aschampion) Index))
    (if (Utilities|Name|NotEqual(Name) _itemkey (Variables|/Game/Blueprints/Components/InventoryComponent.InventoryComponent_C|GetEmptyItemKey (Variables|/Game/Blueprints/Units/MobileUnit/Champions/Champion.Champion_C|GetInventoryComponent _aschampion)))
      (bind _returnvalue (Utilities|GetDataTableRow "/Game/DataTables/ItemDataTable.ItemDataTable" _itemkey)
        (:then
          (Default|RemoveItem (Variables|/Game/Blueprints/Units/MobileUnit/Champions/Champion.Champion_C|GetInventoryComponent _aschampion) Index)
          (Default|AddGold (Variables|/Game/Blueprints/Units/MobileUnit/Champions/Champion.Champion_C|GetInventoryComponent _aschampion) (.SellPrice (Utilities|Struct|BreakItemData _returnvalue))))))))

(event Custom|SendAttack
  (params (TargetUnit :type Unit%20Object%20Reference))
  ;[1 1 1] SendAttack
  (Default|SetCommand (Variables|Client&Server|GetCommandUnit) "NewEnumerator2" "0, 0, 0" TargetUnit))

(event Custom|ReceivePlayerState
  (params (CustomeName :type String) (Team :type bp_Team%20Enum :default "NewEnumerator0") (ChampionKeyName :type Name) (Ready :type Boolean))
  ;[1 1 1] ReceivePlayerState
  (Utilities|GetDataTableRow "/Game/DataTables/UnitDataTable.UnitDataTable" ChampionKeyName
    (:then
      (bind _asbp_my_player_state (Utilities|Casting|CastTobp_MyPlayerState (Variables|Default|GetPlayerState))
        (:then
          (Default|SetPlayerState _asbp_my_player_state (Variables|/Script/OpenMOBA.MyPlayerState|GetplayerTitle _asbp_my_player_state) (Utilities|Select :Index (Variables|/Script/OpenMOBA.MyPlayerState|GetTeamId _asbp_my_player_state) :Option%200 "NewEnumerator1" :Option%201 "NewEnumerator2") ChampionKeyName true))
        (:CastFailed
          (Development|PrintString "bp_MyPlayerController cast to bp_MyPlayerState FAIL"))))))

(event Custom|SendRecallCommand
  ;[1 1 1] SendRecallCommand
  (Default|SetCommand (Variables|Client&Server|GetCommandUnit) "NewEnumerator4" "0, 0, 0"))

(event Custom|BuyItem
  (params (ItemKey :type Name))
  ;[1 1 1] BuyItem
  (if (Utilities|IsCommandUnitValid)
    (bind _aschampion (Utilities|Casting|CastToChampion (Variables|Client&Server|GetCommandUnit)))
    (bind _outactors (Actor|GetAllActorsOfClass "/Game/Blueprints/Fountain/Fountain.Fountain_C"))
    (for _array_element _outactors
      (if (Utilities|Enum|Equal(Enum) (Variables|/Game/Blueprints/Fountain/Fountain.Fountain_C|GetTeam _array_element) (Variables|/Game/Blueprints/Units/Unit.Unit_C|GetTeam (Variables|Client&Server|GetCommandUnit)))
        (bind _distance (CallFunction|GetUnitGroundDistance (Variables|Client&Server|GetCommandUnit) (Transformation|GetActorLocation _array_element)))
        (if (<= _distance 1e+03)
          (bind _returnvalue (Utilities|GetDataTableRow "/Game/DataTables/ItemDataTable.ItemDataTable" ItemKey)
            (:then
              (bind _found (Default|GetEmptySlot (Variables|/Game/Blueprints/Units/MobileUnit/Champions/Champion.Champion_C|GetInventoryComponent _aschampion)))
              (if (and _found (>= (Variables|/Game/Blueprints/Components/InventoryComponent.InventoryComponent_C|GetGold (Variables|/Game/Blueprints/Units/MobileUnit/Champions/Champion.Champion_C|GetInventoryComponent _aschampion)) (.BuyPrice (Utilities|Struct|BreakItemData _returnvalue))))
                (Default|AddGold (Variables|/Game/Blueprints/Units/MobileUnit/Champions/Champion.Champion_C|GetInventoryComponent _aschampion) (- 0 (.BuyPrice (Utilities|Struct|BreakItemData _returnvalue))))
                (Default|AddItem (Variables|/Game/Blueprints/Units/MobileUnit/Champions/Champion.Champion_C|GetInventoryComponent _aschampion) ItemKey)))))))
    (else
      (Development|PrintString "Buy Item - command unit invalid"))))

(event Custom|ClickMiniMap
  (params (Location :type Vector%202D%20Structure))
  (bind (_x _y) (Math|Vector2D|BreakVector2D Location))
  ;[1 1 1] ClickMiniMap
  (Default|SetFocusLocation (Variables|Client|GetClientCamera) (Math|Vector|MakeVector (* _y 5e+03) (* _x 5e+03) 0.0)))

(event Custom|SendIdleCommand
  ;[1 1 1] SendIdleCommand
  (Default|SetCommand (Variables|Client&Server|GetCommandUnit) "NewEnumerator0" "0, 0, 0"))

(event Custom|SendPlayerState
  (params (CustomeName :type String) (Team :type bp_Team%20Enum :default "NewEnumerator0") (ChampionKeyName :type Name) (Ready :type Boolean))
  ;[1 1 1] SendPlayerState
  (CallFunction|ReceivePlayerState CustomeName Team ChampionKeyName Ready))

(event Custom|OpenShopWidget
  ;[1 1 1] Shop
  (bind _visible (CallFunction|IsWidgetVisible "/Game/Blueprints/Widgets/ScoreboardWidget.ScoreboardWidget_C"))
  (if _visible
    (CallFunction|RemoveWidget "/Game/Blueprints/Widgets/ScoreboardWidget.ScoreboardWidget_C")
    (CallFunction|AddWidget "/Game/Blueprints/Widgets/Shop/ShopWidget.ShopWidget_C" 2)
    (else
      (bind _visible_2 (CallFunction|IsWidgetVisible "/Game/Blueprints/Widgets/Shop/ShopWidget.ShopWidget_C"))
      (if _visible_2
        (CallFunction|RemoveWidget "/Game/Blueprints/Widgets/Shop/ShopWidget.ShopWidget_C")
        (else
          (CallFunction|AddWidget "/Game/Blueprints/Widgets/Shop/ShopWidget.ShopWidget_C" 2))))))

(event Custom|SetCenterTextWidget
  (params (CenterText :type Text) (FontSize :type Integer) (Color :type Slate%20Color%20Structure) (Duration :type Float%20%28single-precision%29))
  ;[1 1 1] SetCenterTextWidget
  (bind _returnvalue (UserInterface|CreateWidget "/Game/Blueprints/Widgets/CenterTextWidget.CenterTextWidget_C" self))
  (bind _output_get (Variables|Default|SetCenterTextWidgetRef _returnvalue))
  (UserInterface|Viewport|AddtoViewport _returnvalue 0)
  (Default|SetCenterText _returnvalue CenterText FontSize Color Duration))

(event Custom|UpdateScoreboard
  ;[1 1 1] UpdateScoreboard
  (bind _visible (CallFunction|IsWidgetVisible "/Game/Blueprints/Widgets/ScoreboardWidget.ScoreboardWidget_C"))
  (if _visible
    (bind _widget (CallFunction|GetWidget "/Game/Blueprints/Widgets/ScoreboardWidget.ScoreboardWidget_C"))
    (bind _asscoreboard_widget (Utilities|Casting|CastToScoreboardWidget _widget))
    (Default|UpdatePlayerStates _asscoreboard_widget)))

(event Custom|SendAttackMove
  (params (GoalLocation :type Vector))
  ;[1 1 1] SendAttackMove
  (Default|SetCommand (Variables|Client&Server|GetCommandUnit) "NewEnumerator3" GoalLocation))

(event Custom|Init
  (bind _self self)
  ;[1 1 1] Init
  (Development|PrintString "bp_MyPlayerController Init")
  (bind _returnvalue (UserInterface|CreateWidget "/Game/Blueprints/Widgets/CommandUnitStatusWidget.CommandUnitStatusWidget_C" _self))
  (UserInterface|Viewport|AddtoViewport _returnvalue 0)
  (Input|SetInputModeGameandUI _self 0 "DoNotLock" true)
  (Variables|Default|SetbShowMouseCursor true)
  (Class|MyPlayerController|RefreshChatChannelList _self)
  (bind _asmy_player_state (Utilities|Casting|CastToMyPlayerState (Variables|Default|GetPlayerState)))
  (Class|MyPlayerState|OnReponCustomTextureChange _asmy_player_state))

(event Custom|SendMoveCommand
  (params (GroundLocation :type Vector))
  ;[1 1 1] SendMoveCommand
  (Default|SetCommand (Variables|Client&Server|GetCommandUnit) "NewEnumerator1" GroundLocation))

(event EventBeginPlay)

(event EventTick
  (params (DeltaSeconds :type Float%20%28single-precision%29))
  ;[1 1 1] Tick
  (CallFunction|ScrollCamera))

(event EventRecievePlayerState
  (Development|PrintString "RecieveRecievePlayerState")
  ;[1 1 1] ReceivePlayerState
  (Utilities|GetDataTableRow "/Game/DataTables/UnitDataTable.UnitDataTable" (stale Custom|ReceivePlayerState ChampionKeyName)
    (:then
      (bind _asbp_my_player_state (Utilities|Casting|CastTobp_MyPlayerState (Variables|Default|GetPlayerState))
        (:then
          (Default|SetPlayerState _asbp_my_player_state (Variables|/Script/OpenMOBA.MyPlayerState|GetplayerTitle _asbp_my_player_state) (Utilities|Select :Index (Variables|/Script/OpenMOBA.MyPlayerState|GetTeamId _asbp_my_player_state) :Option%200 "NewEnumerator1" :Option%201 "NewEnumerator2") (stale Custom|ReceivePlayerState ChampionKeyName) true))
        (:CastFailed
          (Development|PrintString "bp_MyPlayerController cast to bp_MyPlayerState FAIL"))))))

(event Input|ActionEvents|InputActionRecall
  (params (Key :type Key%20Structure))
  ;[1 1 1] Recall
  (:Pressed
    (if (Utilities|IsCommandUnitValid)
      (CallFunction|SendRecallCommand))))

(event Input|ActionEvents|InputActionMiddleMouseButtonDown
  (params (Key :type Key%20Structure))
  (bind (_worldlocation _worlddirection) (Game|Player|ConvertMouseLocationToWorldSpace))
  ;[1 1 1] MiddleMouseButtonDown
  (:Pressed
    (if (Utilities|IsCommandUnitValid)
      (bind (_outhit _returnvalue) (Collision|LineTraceByChannel _worldlocation (+ _worldlocation (* _worlddirection 1e+04)) "TraceTypeQuery3" false 0 "None"))
      (if _returnvalue
        (CallFunction|SendAttackMove (.Location (Collision|BreakHitResult _outhit)))))))

(event Input|ActionEvents|InputActionConsumeItem0
  (params (Key :type Key%20Structure))
  ;[1 1 1] ConsumeItem
  (:Pressed
    (CallFunction|SendConsumeItem)))

(event Input|ActionEvents|InputActionScoreboard
  (params (Key :type Key%20Structure))
  ;[1 1 1] Scoreboard - UETOPIA CHANGES - simplified this
  (:Pressed
    (Development|PrintString "Pressed Scoreboard")
    (bind _returnvalue (UserInterface|CreateWidget "/Game/Blueprints/Widgets/ScoreboardWidget.ScoreboardWidget_C"))
    (UserInterface|Viewport|AddtoViewport _returnvalue 0)
    (Variables|Default|SetScoreboardWidgetRef _returnvalue))
  (:Released
    (Development|PrintString "Released Scoreboard")
    (Widget|RemovefromParent (Variables|Default|GetScoreboardWidgetRef))))

(event Input|ActionEvents|InputActionShop
  (params (Key :type Key%20Structure))
  ;[1 1 1] Shop
  (:Pressed
    (CallFunction|OpenShopWidget)))

(event Input|ActionEvents|InputActionRightMouseButtonDown
  (params (Key :type Key%20Structure))
  (bind (_worldlocation _worlddirection) (Game|Player|ConvertMouseLocationToWorldSpace))
  (bind (_worldlocation_2 _worlddirection_2) (Game|Player|ConvertMouseLocationToWorldSpace))
  ;[1 1 1] RightMouseButtonDown
  (:Pressed
    (if (Utilities|IsCommandUnitValid)
      (bind _outhits (Collision|MultiLineTraceByChannel _worldlocation (+ _worldlocation (* _worlddirection 1e+04)) "TraceTypeQuery4" false 0 "None"))
      (Variables|Client|SetAttackUnit false)
      (bind _array_element (Utilities|Array|ForEachLoopwithBreak _outhits :!label _label)
        (:LoopBody
          (bind _asunit (Utilities|Casting|CastToUnit (.HitActor (Collision|BreakHitResult _array_element))))
          (bind _alive (Default|IsAlive _asunit))
          (bind _asbp_my_player_state (Utilities|Casting|CastTobp_MyPlayerState (Variables|Default|GetPlayerState)))
          (bind _vision (Default|GetVision _asunit (Variables|/Game/Blueprints/PlayerState/bp_MyPlayerState.bp_MyPlayerState_C|GetTeam _asbp_my_player_state)))
          (if (Math|Boolean|ANDBoolean (Utilities|Enum|NotEqual(Enum) _vision "NewEnumerator2") (Utilities|Enum|NotEqual(Enum) (Variables|/Game/Blueprints/PlayerState/bp_MyPlayerState.bp_MyPlayerState_C|GetTeam _asbp_my_player_state) (Variables|/Game/Blueprints/Units/Unit.Unit_C|GetTeam _asunit)) _alive)
            (CallFunction|SendAttack _asunit)
            (Variables|Client|SetAttackUnit true)
            (goto _label Break)))
        (:Completed
          (if (not (Variables|Client|GetAttackUnit))
            (bind (_outhit _returnvalue) (Collision|LineTraceByChannel _worldlocation_2 (+ _worldlocation_2 (* _worlddirection_2 1e+04)) "TraceTypeQuery3" false 0 "None"))
            (if _returnvalue
              (CallFunction|SendMoveCommand (.Location (Collision|BreakHitResult _outhit))))))))))

(event Input|ActionEvents|InputActionConsumeItem1
  (params (Key :type Key%20Structure))
  ;[1 1 1] ConsumeItem
  (:Pressed
    (CallFunction|SendConsumeItem 1)))

(event Input|ActionEvents|InputActionConsumeItem2
  (params (Key :type Key%20Structure))
  ;[1 1 1] ConsumeItem
  (:Pressed
    (CallFunction|SendConsumeItem 2)))

(event Input|ActionEvents|InputActionConsumeItem3
  (params (Key :type Key%20Structure))
  ;[1 1 1] ConsumeItem
  (:Pressed
    (CallFunction|SendConsumeItem 3)))

(event Input|ActionEvents|InputActionConsumeItem4
  (params (Key :type Key%20Structure))
  ;[1 1 1] ConsumeItem
  (:Pressed
    (CallFunction|SendConsumeItem 4)))

(event Input|ActionEvents|InputActionConsumeItem5
  (params (Key :type Key%20Structure))
  ;[1 1 1] ConsumeItem
  (:Pressed
    (CallFunction|SendConsumeItem 5)))

(event Custom|CreateCamera
  (bind _commandunit (Variables|Client&Server|GetCommandUnit))
  ;[1 1 1] CreateCamera
  (Utilities|IsValid _commandunit
    (:Is%20Valid
      (if (not (Utilities|IsValid (Variables|Client|GetClientCamera)))
        (bind _returnvalue (Game|SpawnActorfromClass "/Game/Blueprints/Camera/ClientCamera.ClientCamera_C" (Math|Transform|MakeTransform (Transformation|GetActorLocation _commandunit)) "AlwaysSpawn" 0 0))
        (bind _output_get (Variables|Client|SetClientCamera _returnvalue)))
      (Default|Init _output_get (Variables|Client&Server|GetCommandUnit)))))

(event Custom|ScrollCamera
  ;[1 1 1] Tick
  (Utilities|IsValid (Variables|Client|GetClientCamera)
    (:Is%20Valid
      (Utilities|FlowControl|Sequence
        (:then_0
          (if (Game|Player|IsInputKeyDown (Variables|Client|GetScrollUpKey))
            (Default|Scroll (Variables|Client|GetClientCamera) "1000.000000, 0, 0")
            (elif (Game|Player|IsInputKeyDown (Variables|Client|GetScrollDownKey))
              (Default|Scroll (Variables|Client|GetClientCamera) "-1000.000000, 0, 0"))))
        (:then_1
          (if (Game|Player|IsInputKeyDown (Variables|Client|GetScrollRightKey))
            (Default|Scroll (Variables|Client|GetClientCamera) "0.000000,1000.000000, 0")
            (elif (Game|Player|IsInputKeyDown (Variables|Client|GetScrollLeftKey))
              (Default|Scroll (Variables|Client|GetClientCamera) "0.000000,-1000.000000, 0"))))))))

(event Input|ActionEvents|InputActionAutoFollow
  (params (Key :type Key%20Structure))
  (bind _clientcamera (Variables|Client|GetClientCamera))
  ;[1 1 1] AutoFollow
  (:Pressed
    (Utilities|IsValid _clientcamera
      (:Is%20Valid
        (Default|AutoFollowActor _clientcamera)))))

(event Input|ActionEvents|InputActionZoomIn
  (params (Key :type Key%20Structure))
  (bind _clientcamera (Variables|Client|GetClientCamera))
  (:Pressed
    (Utilities|IsValid _clientcamera
      (:Is%20Valid
        (Default|Zoom _clientcamera 1.0)))))

(event Input|ActionEvents|InputActionZoomOut
  (params (Key :type Key%20Structure))
  (bind _clientcamera (Variables|Client|GetClientCamera))
  (:Pressed
    (Utilities|IsValid _clientcamera
      (:Is%20Valid
        (Default|Zoom _clientcamera -1.0)))))

(event EventRemoveWidget
  (params (Class :type User%20Widget%20Class%20Reference))
  ;[1 1 1] RemoveWidget
)

(fn ConstructionScript)

(fn OnRepCommandUnit
  (if (Pawn|IsLocalPlayerController)
    (CallFunction|CreateCamera)))

(fn AddWidget
  (params (Class :type User%20Widget%20Class%20Reference) (ZOrder :type Integer)))

(fn GetWidget
  (params (Class :type User%20Widget%20Class%20Reference)))

(fn IsWidgetVisible
  (params (Class :type User%20Widget%20Class%20Reference)))