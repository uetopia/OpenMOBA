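; Player state for a lobby that holds each player's name, team, champion key and ready flag.
; SetPlayerState applies only changed values, notifying bp_MyGameMode of team and champion changes or triggering its ready check.
; OnRep functions for all four values refresh the scoreboard through the local bp_MyPlayerController.
; CopyProperties carries the values across travel from lobby to game levels, while BeginPlay sets the name from PlayerTitle.
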(event Custom|SetPlayerState
  (params (CustomeName :type String) (Team :type bp_Team%20Enum :default "NewEnumerator0") (ChampionKeyName :type Name) (Ready :type Boolean))
  ;[1 1 1] SetPlayerState
  (Utilities|FlowControl|Sequence
    (:then_0
      (if (Utilities|Enum|NotEqual(Enum) (Variables|Default|GetCustomeName) CustomeName)
        (Variables|Default|SetCustomeName CustomeName)))
    (:then_1
      (if (Utilities|Enum|NotEqual(Enum) (Variables|Default|GetTeam) Team)
        (bind _output_get (Variables|Default|SetTeam Team))
        (bind _asbp_my_game_mode (Utilities|Casting|CastTobp_MyGameMode (Game|GetGameMode)))
        (Default|ChangeTeam _asbp_my_game_mode (Variables|Default|GetPlayerController) _output_get)))
    (:then_2
      (if (Utilities|Name|NotEqual(Name) (Variables|Default|GetChampionKey) ChampionKeyName)
        (bind _output_get_2 (Variables|Default|SetChampionKey ChampionKeyName))
        (bind _asbp_my_game_mode_2 (Utilities|Casting|CastTobp_MyGameMode (Game|GetGameMode)))
        (Default|ChangeChampion _asbp_my_game_mode_2 (Variables|Default|GetPlayerController) _output_get_2)))
    (:then_3
      (if (Math|Boolean|NotEqual(Boolean) (Variables|Default|GetReady) Ready)
        (Variables|Default|SetReady Ready)
        (bind _asbp_my_game_mode_3 (Utilities|Casting|CastTobp_MyGameMode (Game|GetGameMode)))
        (Default|RedyCheck _asbp_my_game_mode_3)))))

(event EventBeginPlay
  (Development|PrintString "bp_MyPlayerState BeginPlay")
  (Variables|Default|SetCustomeName (Variables|Default|GetplayerTitle self)))

(event EventTick
  (params (DeltaSeconds :type Float%20%28single-precision%29)))

(event EventCopyProperties
  (params (NewPlayerState :type Player%20State%20Object%20Reference))
  ;[1 1 1] Travelling from lobby to game levels requires copying these values
  (|CallParentFunction NewPlayerState)
  (Development|PrintString "bp_MyPlayerState Copy Properties")
  (bind _asbp_my_player_state (Utilities|Casting|CastTobp_MyPlayerState NewPlayerState))
  (Variables|bp_MyPlayerState_C|SetReady _asbp_my_player_state (Variables|Default|GetReady))
  (Variables|bp_MyPlayerState_C|SetChampionKey _asbp_my_player_state (Variables|Default|GetChampionKey))
  (Variables|bp_MyPlayerState_C|SetTeam _asbp_my_player_state (Variables|Default|GetTeam))
  (Variables|bp_MyPlayerState_C|SetCustomeName _asbp_my_player_state (Variables|Default|GetCustomeName)))

(fn ConstructionScript)

(fn OnRepCustomeName
  (bind _asbp_my_player_controller (Utilities|Casting|CastTobp_MyPlayerController (Game|GetPlayerController 0)))
  (Default|UpdateScoreboard _asbp_my_player_controller))

(fn OnRepTeam
  (bind _asbp_my_player_controller (Utilities|Casting|CastTobp_MyPlayerController (Game|GetPlayerController 0)))
  (Default|UpdateScoreboard _asbp_my_player_controller))

(fn OnRepChampionKeyName
  (bind _asbp_my_player_controller (Utilities|Casting|CastTobp_MyPlayerController (Game|GetPlayerController 0)))
  (Default|UpdateScoreboard _asbp_my_player_controller))

(fn OnRepReady
  (bind _asbp_my_player_controller (Utilities|Casting|CastTobp_MyPlayerController (Game|GetPlayerController 0)))
  (Default|UpdateScoreboard _asbp_my_player_controller))