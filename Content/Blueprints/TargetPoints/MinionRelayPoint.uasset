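; MinionRelayPoint is a placeable target point, apparently a waypoint for minions, identified by Lane, Number and Team.
; Its construction script sets a text label to the lane name and number with a fixed world rotation.
; It also switches the skeletal mesh material to blue or red to match the team.
; The event graph holds only disabled placeholder events, so the Blueprint adds no runtime logic.
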(event EventBeginPlay)

(event Collision|EventActorBeginOverlap
  (params (OtherActor :type Actor%20Object%20Reference)))

(event EventTick
  (params (DeltaSeconds :type Float%20%28single-precision%29)))

(fn ConstructionScript
  (bind _textrender (Variables|Default|GetTextRender))
  (bind _skeletalmesh (Variables|Default|GetSkeletalMesh))
  (Rendering|Components|TextRender|SetText _textrender (Utilities|Text|FormatText "{0}:{1}" (Utilities|Text|ToText(String) (Utilities|String|EnumtoString (Variables|Default|GetLane))) (Variables|Default|GetNumber)))
  (Transformation|SetWorldRotation _textrender "90.000000,180.000000, 0" false false)
  (switch Utilities|FlowControl|Switch|Switchonbp_Team (Variables|Default|GetTeam)
    (:NewEnumerator1
      (Rendering|Material|SetMaterial _skeletalmesh 0 "/Game/Materials/BlueMaterial.BlueMaterial"))
    (:NewEnumerator2
      (Rendering|Material|SetMaterial _skeletalmesh 0 "/Game/Materials/RedMaterial.RedMaterial"))))